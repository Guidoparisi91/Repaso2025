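; BP_Actor is a timer test actor that loses health over time and destroys itself.
; On BeginPlay it prints VidaActual and starts a looping half-second timer bound to QuitarVida.
; Each tick of that timer subtracts fixed damage through DisminuirVida, prints the new value, and destroys the actor only when health equals exactly zero.
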(event `self.ReceiveBeginPlay`
  (`KismetSystemLibrary.PrintString` (`KismetStringLibrary.Conv_DoubleToString` (`self.VidaActual`)))
  (`KismetSystemLibrary.K2_SetTimerDelegate` (delegate `QuitarVida`) 0.5 true))

(event `QuitarVida`
  (`self.DisminuirVida` 10.0)
  (`KismetSystemLibrary.PrintString` (`KismetStringLibrary.Conv_DoubleToString` (`self.VidaActual`)))
  (if (== (`self.VidaActual`) 0.0)
    (`self.K2_DestroyActor`)))

(fn `DisminuirVida`
  (params (`Daño` :type "Float (double-precision)"))
  (set `self.VidaActual` (- (`self.VidaActual`) `Daño`)))

(fn `UserConstructionScript`)