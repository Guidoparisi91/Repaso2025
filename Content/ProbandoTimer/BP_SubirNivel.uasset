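; BP_SubirNivel is a test actor that simulates automatic leveling through experience gained over time.
; On BeginPlay a looping timer repeatedly fires SubirNivel, which adds experience through SumarExperiencia and prints the total.
; When experience crosses its threshold it resets, the level increments and prints, and the actor destroys itself on reaching the final level.
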(event `self.ReceiveBeginPlay`
  (`KismetSystemLibrary.K2_SetTimerDelegate` (delegate `SubirNivel`) 0.5 true))

(event `SubirNivel`
  (`self.SumarExperiencia` 10)
  (`KismetSystemLibrary.PrintString` (`KismetStringLibrary.Conv_IntToString` (`self.Experiencia`)))
  (if (>= (`self.Experiencia`) 100)
    (set `self.Experiencia` 0)
    (set `self.Nivel` (+ (`self.Nivel`) 1))
    (`KismetSystemLibrary.PrintString` (`KismetStringLibrary.Conv_IntToString` (`self.Nivel`)))
    (if (== (`self.Nivel`) 5)
      (`self.K2_DestroyActor`))))

(fn `SumarExperiencia`
  (params (`Xp a sumar` :type Integer))
  (set `self.Experiencia` (+ (`self.Experiencia`) `Xp a sumar`)))

(fn `UserConstructionScript`)