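; Player character Blueprint that handles movement input and creates the player's HUD.
; On BeginPlay it registers the IMC_PersonajeInputs Enhanced Input context and adds WBP_HUD to the viewport, setting its test text to a hardcoded name.
; IA_Movimiento prints the axis values, then uses nested sign checks to pick one of eight fixed world-space directions for AddMovementInput, independent of camera and stick magnitude.
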(event `self.ReceiveBeginPlay`
  (bind _asplayer_controller (cast `PlayerController` (`self.GetController`)))
  (`EnhancedInputSubsystemInterface.AddMappingContext` (pcsubsystem `EnhancedInputLocalPlayerSubsystem` _asplayer_controller) "/Game/HerenciaYCharacter/BluePrints/Character/Inputs/MappingContext/IMC_PersonajeInputs.IMC_PersonajeInputs" 0 (struct))
  (`self.CreateHud`))

(event `EnhancedInput|/Game/HerenciaYCharacter/BluePrints/Character/Inputs/InputActions/IA_Movimiento`
  (params (ActionValue :type "Vector2D Structure") (ElapsedSeconds :type "Float (double-precision)") (TriggeredSeconds :type "Float (double-precision)") (InputAction :type "InputAction Object Reference" :default "/Game/HerenciaYCharacter/BluePrints/Character/Inputs/InputActions/IA_Movimiento.IA_Movimiento"))
  (:`Triggered`
    (`KismetSystemLibrary.PrintString` (`KismetStringLibrary.Concat_StrStr` "valor x " (`KismetStringLibrary.Conv_DoubleToString` ActionValue_X) " \nvalor y " (`KismetStringLibrary.Conv_DoubleToString` ActionValue_Y)))
    (if (and (== ActionValue_X 0.0) (> ActionValue_Y 0.0))
      (`self.AddMovementInput` (0.0 -1.0 0.0))
      (elif (and (< ActionValue_X 0.0) (> ActionValue_Y 0.0))
        (`self.AddMovementInput` (1.0 -1.0 0.0))
        (elif (and (< ActionValue_X 0.0) (== ActionValue_Y 0.0))
          (`self.AddMovementInput` (1.0 0.0 0.0))
          (elif (and (< ActionValue_X 0.0) (< ActionValue_Y 0.0))
            (`self.AddMovementInput` (1.0 1.0 0.0))
            (elif (and (== ActionValue_X 0.0) (< ActionValue_Y 0.0))
              (`self.AddMovementInput` (0.0 1.0 0.0))
              (elif (and (> ActionValue_X 0.0) (< ActionValue_Y 0.0))
                (`self.AddMovementInput` (-1.0 1.0 0.0))
                (elif (and (> ActionValue_X 0.0) (== ActionValue_Y 0.0))
                  (`self.AddMovementInput` (-1.0 0.0 0.0))
                  (elif (and (> ActionValue_X 0.0) (> ActionValue_Y 0.0))
                    (`self.AddMovementInput` (-1.0 -1.0 0.0))))))))))))

(fn `CreateHud`
  (bind _asplayer_controller (cast `PlayerController` (`self.GetController`)))
  (bind _returnvalue (`|CreateWidget` "/Game/HerenciaYCharacter/Sprites/WBP_HUD.WBP_HUD_C" _asplayer_controller))
  (`UserWidget.AddToViewport` _returnvalue 0)
  (bind _output_get (set `self.TextoPrincipal` _returnvalue))
  (set `TextBlock.Text` "Guido" (`/Game/HerenciaYCharacter/Sprites/WBP_HUD.Text_Prueba` _output_get)))

(fn `UserConstructionScript`)